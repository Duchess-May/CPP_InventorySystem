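; Player controller Blueprint that drops inventory items back into the world in front of the player.
; DropItem looks up the item's row in its data table and spawns that row's actor class, passing the item data in as ItemInfo.
; ForwardFromPlayer supplies the spawn transform, a point a set distance along the pawn's forward vector with the pawn's rotation.
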(event EventBeginPlay)

(event EventTick
  (params (DeltaSeconds :type Float%20%28single-precision%29)))

(fn ConstructionScript)

(fn DropItem
  (params (ItemData :type S%20Slots%20Structure))
  (bind _item (Utilities|Struct|BreakS_Slots ItemData))
  (bind (_returnvalue _returnvalue2) (CallFunction|ForwardfromPlayer 1.5e+02))
  (bind (_datatable _rowname) (Utilities|Struct|BreakDataTableRowHandle _item))
  (bind _returnvalue_2 (Utilities|GetDataTableRow _datatable _rowname)
    (:then
      (Game|SpawnActorfromClass (.ActorClass (Utilities|Struct|BreakS_Inventory _returnvalue_2)) (Math|Transform|MakeTransform _returnvalue _returnvalue2 "1.000000,1.000000,1.000000") "Undefined" "MultiplyWithRoot" 0 ItemData 0)
      (return))))

(fn ForwardfromPlayer
  (params (Distance :type Float%20%28double-precision%29))
  (bind _returnvalue (Game|Player|GetPlayerPawn 0))
  (return (+ (Transformation|GetActorLocation _returnvalue) (* (Transformation|GetActorForwardVector _returnvalue) Distance)) (Transformation|GetActorRotation _returnvalue)))