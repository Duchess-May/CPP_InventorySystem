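; BP_CommonLibrary is a shared helper library for reaching the project's player objects and inventory data.
; ProjectPlayerCharacter and ProjectPlayerController return player index 0's pawn and controller, cast to BP_Player and BP_PlayerController.
; GetInventoryDataTableRow looks up a named row in the player's InventoryData table, returning it only when the table is valid and the row is found.
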(fn ProjectPlayerCharacter
  (bind _asbp_player (Utilities|Casting|CastToBP_Player (Game|Player|GetPlayerPawn 0)))
  (return _asbp_player))

(fn ProjectPlayerController
  (bind _asbp_player_controller (Utilities|Casting|CastToBP_PlayerController (Game|GetPlayerController 0)))
  (return _asbp_player_controller))

(fn GetInventoryDataTableRow
  (params (RowName :type Name))
  (bind _inventorydata (Variables|/Game/Blueprints/Characters/BP_Player.BP_Player_C|GetInventoryData (CallFunction|ProjectPlayerCharacter))
    (:then
      (bind _returnvalue (Utilities|GetDataTableRow _inventorydata RowName)
        (:then
          (return _returnvalue))))
    (:else)))