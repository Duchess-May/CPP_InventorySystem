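; Player character Blueprint that handles interacting with nearby tagged objects and showing the inventory HUD.
; The I key toggles the inventory widget, and RefreshInventory rebuilds it by removing and recreating it.
; Completing IA_Interact runs a sphere trace around the player, filters hits by tag and selects the closest.
; The trace branches on that actor's first tag, but only the Pickup branch is wired, sending InteractMessage to it.
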(event Custom|RefreshInventory
  (Utilities|RemoveInventoryHUD)
  (Utilities|AddInventoryHUD))

(event Input|EnhancedActionEvents|EnhancedInputActionIA_Interact
  (params (ActionValue :type Boolean) (ElapsedSeconds :type Float%20%28double-precision%29) (TriggeredSeconds :type Float%20%28double-precision%29) (InputAction :type Input%20Action%20Object%20Reference :default "/Game/Static/Input/Actions/IA_Interact.IA_Interact"))
  (:Completed
    (bind _interactible (Utilities|SphereTraceforInteractibles)
      (:Pickup
        (Class|BPIInteract|Interact(Message) _interactible self)))))

(event EventTick
  (params (DeltaSeconds :type Float%20%28single-precision%29)))

(event Input|KeyboardEvents|I
  (params (Key :type Key%20Structure :default "None"))
  (:Released
    (Utilities|FlowControl|FlipFlop
      (:A
        (Utilities|AddInventoryHUD))
      (:B
        (Utilities|RemoveInventoryHUD)))))

(fn ConstructionScript
  (|CallParentFunction))

(fn GetClosestInteractiononInteract
  (params (Array :type Array%20of%20Hit%20Result%20Structures) (ValidCollision :type Boolean))
  (if ValidCollision
    ;[0 0 0 1 12] Set same as pickup sphere trace radius (+50%)
    (LocalVariables|SetLocalDistance 3e+02)
    (for _array_element Array
      (Utilities|IsInteractiblebyTag? (.HitActor (Collision|BreakHitResult _array_element))
        (:true
          (Utilities|Array|AddUnique (LocalVariables|GetLocalActors) (.HitActor (Collision|BreakHitResult _array_element))))))
    (bind (_array_element_2 _array_index) (Utilities|Array|ForEachLoopwithBreak (LocalVariables|GetLocalActors))
      (:LoopBody
        (if (< (Transformation|GetDistanceTo _array_element_2) (LocalVariables|GetLocalDistance))
          (LocalVariables|SetLocalDistance (Transformation|GetDistanceTo _array_element_2))
          (LocalVariables|SetLocalClosestInteractible _array_element_2)
          (LocalVariables|SetLocalClosestIndex _array_index)))
      (:Completed
        (bind _array_element_3 (Utilities|Array|ForEachLoopwithBreak (LocalVariables|GetLocalActors))
          (:LoopBody
            (Utilities|Casting|CastToBP_ItemMaster _array_element_3))
          (:Completed
            (return (LocalVariables|GetLocalClosestInteractible) (LocalVariables|GetLocalDistance))))))
    (else
      (return 0 0.0))))